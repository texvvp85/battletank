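; Player tank Blueprint whose shown logic handles camera look input.
; The horizontal look axis adds local yaw to the Gimble component, while the vertical axis adds local pitch to the SpringArm.
; Splitting yaw and pitch across two components avoids unwanted roll, and both inputs scale by Sensitivity and world delta seconds, with no pitch clamp in the graph.
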(event `InputAxis|LookRight/Left`
  (params (AxisValue :type "Float (single-precision)"))
  ;[1 1 1] Look
  (`SceneComponent.K2_AddLocalRotation` (`self.Gimble`) (`KismetMathLibrary.MakeRotator` 0.0 0.0 (* AxisValue (`GameplayStatics.GetWorldDeltaSeconds`) (`self.Sensitivity`))) false false))

(event `InputAxis|LookUp/Down`
  (params (AxisValue :type "Float (single-precision)"))
  ;[1 1 1] Look
  (`SceneComponent.K2_AddLocalRotation` (`self.SpringArm`) (`KismetMathLibrary.MakeRotator` 0.0 (* AxisValue (`GameplayStatics.GetWorldDeltaSeconds`) (`self.Sensitivity`))) false false))

(fn `UserConstructionScript`)